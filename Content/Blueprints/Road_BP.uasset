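; Road tile Blueprint for a road that extends as the player pawn advances.
; When an HCF6Pawn overlaps EndTrigger, it has the game mode add a road tile, then destroys its attached opponent after a short delay.
; The construction script collects the left and right points into RoadPoints, and GetAttachTransform exposes the AttachPoint world transform.
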(event OnComponentBeginOverlap(EndTrigger)
  (params (OverlappedComponent :type Primitive%20Component%20Object%20Reference) (OtherActor :type Actor%20Object%20Reference) (OtherComp :type Primitive%20Component%20Object%20Reference) (OtherBodyIndex :type Integer) (bFromSweep :type Boolean) (SweepResult :type Hit%20Result%20Structure%20%28by%20ref%29))
  (Utilities|Casting|CastToHCF6Pawn OtherActor)
  (bind _ashcf6game_mode_bp (Utilities|Casting|CastToHCF6GameMode_BP (Game|GetGameMode)))
  (Default|AddRoadTile _ashcf6game_mode_bp)
  (Utilities|FlowControl|Delay 2.0)
  (Actor|DestroyActor (Variables|Default|GetAttachedOpponentReference)))

(event EventBeginPlay)

(event Collision|EventActorBeginOverlap
  (params (OtherActor :type Actor%20Object%20Reference)))

(event EventTick
  (params (DeltaSeconds :type Float%20%28single-precision%29)))

(fn ConstructionScript
  (bind _roadpoints (Variables|Default|GetRoadPoints))
  (Utilities|Array|Add _roadpoints (Variables|Default|GetLeftPoint))
  (Utilities|Array|Add _roadpoints (Variables|Default|GetRightPoint)))

(fn GetAttachTransform
  (return (Transformation|GetWorldTransform (Variables|Default|GetAttachPoint))))