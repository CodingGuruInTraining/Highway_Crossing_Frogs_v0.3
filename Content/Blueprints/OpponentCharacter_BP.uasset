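; Opponent character that paces back and forth between the left and right edge points of its owning Road_BP.
; Tick offsets the capsule along local Y until its world Y nears the edge it faces, then flips the facing flags.
; Each turn pauses movement while RotatingMovement runs for a one-second delay.
; Any capsule hit or overlap switches the mesh to physics simulation; several older rotation experiments remain unconnected.
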(event OnComponentHit(CapsuleComponent)
  (params (HitComponent :type Primitive%20Component%20Object%20Reference) (OtherActor :type Actor%20Object%20Reference) (OtherComp :type Primitive%20Component%20Object%20Reference) (NormalImpulse :type Vector :default "0, 0, 0") (Hit :type Hit%20Result%20Structure%20%28by%20ref%29))
  (Physics|SetSimulatePhysics (Variables|Character|GetMesh) true))

(event OnComponentBeginOverlap(CapsuleComponent)
  (params (OverlappedComponent :type Primitive%20Component%20Object%20Reference) (OtherActor :type Actor%20Object%20Reference) (OtherComp :type Primitive%20Component%20Object%20Reference) (OtherBodyIndex :type Integer) (bFromSweep :type Boolean) (SweepResult :type Hit%20Result%20Structure%20%28by%20ref%29))
  (Physics|SetSimulatePhysics (Variables|Character|GetMesh) true))

(event Custom|TurnAround
  (bind _rotatingmovement (Variables|Default|GetRotatingMovement))
  (Components|Activation|SetActive _rotatingmovement true false)
  (Utilities|FlowControl|Delay 1.0)
  (Components|Activation|SetActive _rotatingmovement false false)
  (Variables|Default|SetTurning false))

(event EventBeginPlay
  (CallFunction|InitVariables))

(event EventTick
  (params (DeltaSeconds :type Float%20%28single-precision%29))
  (Variables|Default|SetDeltaSeconds DeltaSeconds)
  (if (not (Variables|Default|GetTurning))
    (if (Variables|Default|GetFacingLeft)
      (bind _returnvalue (CallFunction|IsatLeftEdge))
      (if _returnvalue
        (CallFunction|ChangeDirection :!label _label)
        (else
          (CallFunction|MoveLocation :!label _label_2)))
      (elif (Variables|Default|GetFacingRight)
        (bind _returnvalue_2 (CallFunction|IsatRightEdge))
        (if _returnvalue_2
          (goto _label)
          (else
            (goto _label_2)))))))

(fn ConstructionScript)

(fn SetInterpPoints)

(fn InitVariables
  (bind _asroad_bp (Utilities|Casting|CastToRoad_BP (Components|GetOwner)))
  (Variables|Default|SetRoadReference _asroad_bp)
  (Variables|Default|SetLeftLocation (Transformation|GetWorldLocation (Variables|/Game/Blueprints/Road_BP.Road_BP_C|GetLeftPoint (Variables|Default|GetRoadReference))))
  (Variables|Default|SetRightLocation (Transformation|GetWorldLocation (Variables|/Game/Blueprints/Road_BP.Road_BP_C|GetRightPoint (Variables|Default|GetRoadReference))))
  (Variables|Default|SetLeftTransform (Transformation|GetWorldTransform (Variables|/Game/Blueprints/Road_BP.Road_BP_C|GetLeftPoint (Variables|Default|GetRoadReference))))
  (Variables|Default|SetRightTransform (Transformation|GetWorldTransform (Variables|/Game/Blueprints/Road_BP.Road_BP_C|GetRightPoint (Variables|Default|GetRoadReference))))
  (Utilities|Array|Add (Variables|Default|GetDirectionsArray) (Variables|Default|GetFacingLeft))
  (Utilities|Array|Add (Variables|Default|GetDirectionsArray) (Variables|Default|GetFacingRight))
  (Components|Activation|Deactivate (Variables|Default|GetRotatingMovement)))

(fn ChangeDirection
  (if (Variables|Default|GetFacingLeft)
    (Variables|Default|SetFacingLeft false)
    (Variables|Default|SetFacingRight true)
    (else
      (Variables|Default|SetFacingLeft true)
      (Variables|Default|SetFacingRight false)))
  (Variables|Default|SetTurning true)
  (CallFunction|TurnAround))

(fn MoveLocation
  (Transformation|AddLocalOffset (Variables|Collision|GetCapsuleComponent) (* (Math|Vector|MakeVector 0.0 (Variables|Default|GetMoveSpeed) 0.0) (Variables|Default|GetDeltaSeconds)) false false))

(fn IsatLeftEdge
  (return (Math|Float|NearlyEqual(Float) (.Y (Math|Vector|BreakVector (Transformation|GetWorldLocation (Variables|Collision|GetCapsuleComponent)))) (.Y (Math|Vector|BreakVector (Math|Transform|TransformLocation (Variables|Default|GetLeftTransform) (Variables|Default|GetLeftLocation)))) 5e+01)))

(fn IsatRightEdge
  (return (Math|Float|NearlyEqual(Float) (.Y (Math|Vector|BreakVector (Transformation|GetWorldLocation (Variables|Collision|GetCapsuleComponent)))) (.Y (Math|Vector|BreakVector (Math|Transform|TransformLocation (Variables|Default|GetRightTransform) (Variables|Default|GetRightLocation)))) 5e+01)))

(fn ChangeSpeed
  (Variables|Default|SetMoveSpeed (* (Variables|Default|GetMoveSpeed) -1.0)))