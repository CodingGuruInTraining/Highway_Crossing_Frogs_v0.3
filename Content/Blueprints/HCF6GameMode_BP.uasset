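; Game mode that builds the road from chained tiles, starting with ten at BeginPlay, and populates each with an opponent.
; AddRoadTile spawns Road_BP at SpawnPoint, then advances SpawnPoint to that tile's attach transform.
; It spawns an OpponentCharacter_BP owned by the tile at one of its random road points and links the two.
; PickDirection randomly sets the opponent facing left or right, rotating left-facing ones 180 degrees.
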(event EventBeginPlay
  (for _index (range 0 9)
    (CallFunction|AddRoadTile)))

(fn ConstructionScript)

(fn AddRoadTile
  (bind _returnvalue (Game|SpawnActorfromClass "/Game/Blueprints/Road_BP.Road_BP_C" (Variables|Default|GetSpawnPoint) "Undefined" 0 0))
  (bind _output_get (Variables|Default|SetRoadReference _returnvalue))
  (bind _returnvalue_2 (Default|GetAttachTransform _output_get))
  (Variables|Default|SetSpawnPoint _returnvalue_2)
  (bind _returnvalue_3 (CallFunction|PickSpawnLocation))
  (Utilities|Array|Add (Variables|Default|GetAllPoints) _returnvalue_3)
  (bind _returnvalue_4 (Game|SpawnActorfromClass "/Game/Blueprints/OpponentCharacter_BP.OpponentCharacter_BP_C" _returnvalue_3 "Undefined" (Variables|Default|GetRoadReference) 0))
  (Variables|Default|SetOpponentReference _returnvalue_4)
  (Utilities|Array|Add (Variables|Default|GetActorsArray) (Variables|Default|GetOpponentReference))
  (CallFunction|PickDirection)
  (Variables|/Game/Blueprints/Road_BP.Road_BP_C|SetAttachedOpponentReference (Variables|Default|GetRoadReference) (Variables|Default|GetOpponentReference)))

(fn PickSpawnLocation
  (bind _roadreference (Variables|Default|GetRoadReference))
  (bind _roadpoints (Variables|/Game/Blueprints/Road_BP.Road_BP_C|GetRoadPoints _roadreference))
  (return (Transformation|GetWorldTransform (Utilities|Array|Get(acopy) _roadpoints (Math|Random|RandomIntegerinRange 0 (Utilities|Array|LastIndex _roadpoints))))))

(fn PickDirection
  (bind _opponentreference (Variables|Default|GetOpponentReference))
  (if (== (Math|Random|RandomIntegerinRange 0 1) 0)
    (Variables|/Game/Blueprints/OpponentCharacter_BP.OpponentCharacter_BP_C|SetFacingLeft _opponentreference false)
    (Variables|/Game/Blueprints/OpponentCharacter_BP.OpponentCharacter_BP_C|SetFacingRight _opponentreference true)
    (else
      (Variables|/Game/Blueprints/OpponentCharacter_BP.OpponentCharacter_BP_C|SetFacingLeft _opponentreference true)
      (Variables|/Game/Blueprints/OpponentCharacter_BP.OpponentCharacter_BP_C|SetFacingRight _opponentreference false)
      (Transformation|AddActorLocalRotation _opponentreference "0,180.000000, 0" false false))))